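; BP_PlayerPawn is the player pawn, with a debug control that steers wind in the pollution simulation.
; Holding the P debug key opens a Gate on Tick, which looks up BP_PollutionManager and calls SetWind every frame.
; Wind direction is the camera forward vector's unnormalized XY, and strength is its length, so wind weakens as the view pitches up or down.
; The vector is also printed for debugging.
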(event EventTick
  (params (DeltaSeconds :type Float%20%28single-precision%29))
  (bind _returnvalue (Game|GetPlayerCameraManager 0))
  (bind _returnvalue_2 (Camera|GetCameraRotation _returnvalue))
  (bind _returnvalue_3 (Math|Vector|GetForwardVector _returnvalue_2))
  (bind _returnvalue_4 (Math|Vector2D|MakeVector2D (.x _returnvalue_3) (.y _returnvalue_3)))
  (Utilities|FlowControl|Gate true
    (:Exit
      (bind _returnvalue_5 (Actor|GetActorOfClass "/Game/BP_PollutionManager.BP_PollutionManager_C"))
      (Class|PollutionManager|SetWind _returnvalue_5 _returnvalue_4 (Math|Vector2D|Vector2DLength _returnvalue_4))
      (Development|PrintString (Utilities|String|ToString(Vector2d) _returnvalue_4) true true "(R=0.000000,G=0.660000,B=1.000000,A=1.000000)" 2.0 "d"))))

(event Input|KeyboardEvents|DebugKeyP
  (params (Key :type Key%20Structure :default "None") (ActionValue :type Input%20Action%20Value%20Structure))
  (bind _returnvalue (Game|GetPlayerCameraManager 0))
  (bind _returnvalue_2 (Camera|GetCameraRotation _returnvalue))
  (bind _returnvalue_3 (Math|Vector|GetForwardVector _returnvalue_2))
  (bind _returnvalue_4 (Math|Vector2D|MakeVector2D (.x _returnvalue_3) (.y _returnvalue_3)))
  (:Pressed
    (Utilities|FlowControl|Gate true) ; enters at Open
  )
  (:Released
    (Utilities|FlowControl|Gate true) ; enters at Close
  ))

(fn ConstructionScript)